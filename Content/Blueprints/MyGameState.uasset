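; MyGameState is a game state Blueprint that runs a match countdown and opens the end-game menu when time runs out.
; On authority, a looping one-second timer calls EndGame, which decrements Time and then calls ShowEndGameMenu.
; Once Time drops below one, that event clears the timers and calls ShowEndGameMenu on player controller 0, cast to MyPlayerController.
; Both OnRep functions are empty.
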(event `self.ReceiveBeginPlay`
  (`/Engine/EditorBlueprintResources/ActorMacros.Switch Has Authority`
    (:`Authority`
      (`KismetSystemLibrary.K2_SetTimer` null "EndGame" 1.0 true))))

(event `ShowEndGameMenu`
  (if (< (stale `EndGame` _output_get) 1)
    (`KismetSystemLibrary.K2_ClearTimer` null "EndGame")
    (`KismetSystemLibrary.K2_ClearTimer` null "ShowEndGameMenu")
    (bind _asmy_player_controller (cast `/Game/Blueprints/MyPlayerController` (`GameplayStatics.GetPlayerController` 0)))
    (`/Game/Blueprints/MyPlayerController.ShowEndGameMenu` _asmy_player_controller)))

(event `EndGame`
  (bind _output_get (set `self.Time` (- (`self.Time`) 1)))
  (`self.ShowEndGameMenu`))

(fn `OnRep_GameStartTimer`)

(fn `OnRep_RandomTimerValue1`)

(fn `UserConstructionScript`)