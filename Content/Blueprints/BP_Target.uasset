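; BP_Target is a shootable target that loses health from any damage and awards a point when destroyed.
; At zero health, the authority plays a quietened sound at the target's location, then destroys it and spawns a new BP_Target at a random position within fixed world-space bounds.
; It then increments the score on the damage instigator's MyPlayerState.
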(event `Blink`
  ;[0 0 0] Take Damage
  (`self.K2_DestroyActor`)
  (`|SpawnActorFromClass` "BP_Target_C" (`KismetMathLibrary.MakeTransform` (`KismetMathLibrary.MakeVector` (`KismetMathLibrary.RandomFloatInRange` -300.0 300.0) (`KismetMathLibrary.RandomFloatInRange` 0.0 100.0) (`KismetMathLibrary.RandomFloatInRange` 30.0 300.0))) "Undefined" "OverrideRootScale" null null))

(event `AnimSound`
  ;[0 0 0] Take Damage
  ;;[0 1 0] Sound
  (`GameplayStatics.PlaySoundAtLocation` "/Game/Sounds/Randomize_03.Randomize_03" (`self.K2_GetActorLocation`) (struct) (* (`self.VolumeMultiplier`) 0.1) 1.0 0.0 null null null))

(event `self.ReceiveAnyDamage`
  (params (Damage :type "Float (single-precision)") (DamageType :type "DamageType Object Reference") (InstigatedBy :type "Controller Object Reference") (DamageCauser :type "Actor Object Reference"))
  ;[0 0 0] Take Damage
  (set `self.Health` (- (`self.Health`) (`KismetMathLibrary.FFloor` Damage)))
  (if (<= (`self.Health`) 0)
    (`/Engine/EditorBlueprintResources/ActorMacros.Switch Has Authority`
      (:`Authority`
        (`self.AnimSound`)
        (`self.Blink`)
        (bind _asmy_player_state (cast `/Game/Blueprints/MyPlayerState` (`Controller.PlayerState` InstigatedBy)))
        (`/Game/Blueprints/MyPlayerState.IncrementScore` _asmy_player_state)))))

(fn `UserConstructionScript`)